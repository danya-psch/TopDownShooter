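; AI controller for enemy characters that starts the BT_EnemyAI behavior tree on BeginPlay.
; Custom events move the pawn toward player 0 (TrackHero) and snap it to a look-at rotation toward that player (Rotate), but nothing in this graph calls them.
; AttackPlayer is empty; the weapon trigger and looping timers for TrackHero and Rotate are disconnected leftovers, as is an unused interpolated rotation.
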(event Custom|AttackPlayer)

(event Custom|Rotate
  (Transformation|SetActorRotation (Pawn|GetControlledPawn) (Math|Rotator|FindLookatRotation (Transformation|GetActorLocation) (Transformation|GetActorLocation (Game|GetPlayerCharacter 0)))))

(event Custom|TrackHero
  (AI|AIMoveTo (Pawn|GetControlledPawn) "0, 0, 0" (Game|GetPlayerCharacter 0) 3e+02 false))

(event EventBeginPlay
  (AI|RunBehaviorTree "/Game/Blueprints/EnemyAI/BT_EnemyAI.BT_EnemyAI"))

(fn ConstructionScript)