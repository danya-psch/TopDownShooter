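; Behavior Tree task that finds the player's HeroCharacter for enemy AI to target.
; On execute it casts player controller 0's pawn, stores it in the Player blackboard key and finishes successfully.
; If the cast fails, FinishExecute is never called.
; A disconnected branch that would store a random TargetPoint in the Enemy key never runs.
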(event EventReceiveExecuteAI
  (params (OwnerController :type AI%20Controller%20Object%20Reference) (ControlledPawn :type Pawn%20Object%20Reference))
  (bind _ashero_character (Utilities|Casting|CastToHeroCharacter (Pawn|GetControlledPawn (Game|GetPlayerController 0))))
  (Class|BTFunctionLibrary|SetBlackboardValueasObject (Variables|Default|GetPlayer) _ashero_character)
  (AI|BehaviorTree|FinishExecute true))