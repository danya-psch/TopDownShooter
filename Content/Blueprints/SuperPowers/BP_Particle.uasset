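; BP_Particle is a super-power area effect that repeatedly changes the health of characters inside it, then destroys itself.
; Overlap events maintain a Characters list of BaseCharacters carrying the configured Tag, skipping those tagged inSpawner on entry.
; On BeginPlay a ForLoopWithDelay macro runs timed ticks, each sending AffectHealthMessage with Delta to every listed character, and destroys the actor on completion.
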(event Custom|CalcHealth
  (for _array_element (Variables|Default|GetCharacters)
    (Class|Damageable|AffectHealth(Message) _array_element (Variables|Default|GetDelta))))

(event Collision|EventActorEndOverlap
  (params (OtherActor :type Actor%20Object%20Reference))
  (bind _asbase_character (Utilities|Casting|CastToBaseCharacter OtherActor))
  (Utilities|Array|RemoveItem (Variables|Default|GetCharacters) _asbase_character))

(event Collision|EventActorBeginOverlap
  (params (OtherActor :type Actor%20Object%20Reference))
  (if (and (Actor|ActorHasTag OtherActor (Variables|Default|GetTag)) (not (Actor|ActorHasTag OtherActor "inSpawner")))
    (bind _asbase_character (Utilities|Casting|CastToBaseCharacter OtherActor))
    (if (not (Utilities|Array|ContainsItem (Variables|Default|GetCharacters) _asbase_character))
      (Utilities|Array|Add (Variables|Default|GetCharacters) _asbase_character))))

(event EventTick
  (params (DeltaSeconds :type Float%20%28single-precision%29)))

(event EventBeginPlay
  (Utilities|ForLoopwithDelay 0 (Variables|Default|GetNumberOfCalls) (Variables|Default|GetDelay)
    (:LoopBody
      (CallFunction|CalcHealth))
    (:Completed
      (Actor|DestroyActor))))

(fn ConstructionScript)