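; Door actor that slides open when its Move event is called, with no logic for closing.
; Move starts a looping timer on Opening, which steps the static mesh in world space opposite the Arrow component's forward vector.
; The timer clears once the mesh's world location is far enough from StartLocation, which BeginPlay captures as a relative location.
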(event Custom|Move
  (Utilities|Time|SetTimerbyFunctionName 0 "Opening" 0.1 true))

(event Custom|Opening
  (bind _staticmesh (Variables|Default|GetStaticMesh))
  (Transformation|SetWorldLocation _staticmesh (+ (Transformation|GetWorldLocation _staticmesh) (* (Math|Vector|Normalize (Math|Rotator|GetRotationXVector (Transformation|GetWorldRotation (Variables|Default|GetArrow)))) -10)) false false)
  (if (>= (Math|Vector|VectorLength (- (Transformation|GetWorldLocation (Variables|Default|GetStaticMesh)) (Variables|Default|GetStartLocation))) 6e+02)
    (Utilities|Time|ClearTimerbyFunctionName 0 "Opening")))

(event EventBeginPlay
  (Variables|Default|SetStartLocation (Variables|/Script/Engine.SceneComponent|GetRelativeLocation (Variables|Default|GetStaticMesh))))

(event Collision|EventActorBeginOverlap
  (params (OtherActor :type Actor%20Object%20Reference)))

(fn ConstructionScript)