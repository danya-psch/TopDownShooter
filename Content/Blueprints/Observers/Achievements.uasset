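; Achievements observer Blueprint that tracks enemy deaths as progress toward kill-count achievements.
; OnNotify switches on the incoming event, increments a dead-enemy counter, and calls Unlock when that count hits either of two milestones.
; Unlock only checks whether the achievement is already in the Achievements collection; nothing is recorded or awarded yet.
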(event EventBeginPlay
  (|CallParentFunction) ; This node is disabled and will not be called.\nDrag off pins to build functionality.
)

(event Collision|EventActorBeginOverlap
  (params (OtherActor :type Actor%20Object%20Reference))
  (|CallParentFunction OtherActor) ; This node is disabled and will not be called.\nDrag off pins to build functionality.
)

(event EventTick
  (params (DeltaSeconds :type Float%20%28single-precision%29))
  (|CallParentFunction DeltaSeconds) ; This node is disabled and will not be called.\nDrag off pins to build functionality.
)

(event EventOnNotify
  (params (Event :type E_ObserverEvent%20Enum :default "NewEnumerator0"))
  (switch Utilities|FlowControl|Switch|SwitchonE_ObserverEvent Event
    (:NewEnumerator0
      (bind _output_get (Variables|Default|SetDeadEnemies (+ (Variables|Default|GetDeadEnemies) 1)))
      (switch string (Utilities|String|ToString(Integer) _output_get)
        (:5
          (CallFunction|Unlock "NewEnumerator0"))
        (:10
          (CallFunction|Unlock "NewEnumerator1"))))))

(fn ConstructionScript
  (|CallParentFunction))

(fn Unlock
  (params (Achievement :type E_Achievement%20Enum :default "NewEnumerator0"))
  (if (not (Utilities|Map|Contains (Variables|Default|GetAchievements) Achievement))
    _))