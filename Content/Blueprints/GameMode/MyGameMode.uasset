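; Game mode that opens level menus, starts matches, relays achievement and superpower changes to the HUD, and plays the ending sequence.
; StartGame builds and possesses the hero through a Builder, creates the HUD and places spawners from SpawnData.
; Spawners share one cached template enemy per type, created by a factory method on first use.
; IncrementScore adds score, counts kills and moves Doors whose kill threshold matches the count.
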(event Custom|SuperPowerChange
  (params (SuperPowerName :type E_SuperPowerName%20Enum :default "EHeal"))
  (Default|SuperPowerChange (Variables|Default|GetActiveHUD) SuperPowerName))

(event Custom|EndOfTheGame
  (bind _returnvalue (Sequencer|Player|CreateLevelSequencePlayer "/Game/Cinematics/EndOfGameLevelSequence.EndOfGameLevelSequence"))
  (Viewport|RemoveAllWidgets)
  (Sequencer|Player|Play _returnvalue :!class /Script/MovieScene.MovieSceneSequencePlayer)
  (Utilities|FlowControl|Delay 5.0)
  (Game|OpenLevel(byName) "MainMenuMap"))

(event Custom|ShowAchievement
  (params (NewParam :type Integer))
  (Default|ShowAchievement (Variables|Default|GetActiveHUD) (Utilities|Enum|ByteToEnumE_Achievement (Math|Conversions|ToByte(Integer) NewParam))))

(event Custom|StartGame
  (CallFunction|CreatingSpawners (Variables|Default|GetSpawnData))
  (bind _returnvalue (UserInterface|CreateWidget "/Game/Blueprints/Widgets/MyHUD.MyHUD_C"))
  (UserInterface|Viewport|AddtoViewport _returnvalue 0)
  (Variables|Default|SetActiveHUD _returnvalue)
  (bind _herocharacter (CallFunction|GenerateHeroCharacter (Variables|Default|GetStart)))
  (Pawn|Possess (Game|GetPlayerController 0) _herocharacter)
  (Actor|DestroyActor (Variables|Default|GetBuilder)))

(event Custom|ChangeLevel
  (params (LevelName :type Name))
  (switch name LevelName
    (:ArenaMap
      (bind _returnvalue (UserInterface|CreateWidget "/Game/Blueprints/Widgets/CharacterSelectMenuWidget.CharacterSelectMenuWidget_C" :!label _label))
      (UserInterface|Viewport|AddtoViewport _returnvalue 0))
    (:MainMenuMap
      (bind _returnvalue_2 (UserInterface|CreateWidget "/Game/Blueprints/Widgets/MainMenuWidget.MainMenuWidget_C"))
      (UserInterface|Viewport|AddtoViewport _returnvalue_2 0))
    (:MainMap
      (goto _label))))

(event Custom|IncrementScore
  (params (DeltaScore :type Integer))
  (Variables|Default|SetScore (+ DeltaScore (Variables|Default|GetScore)))
  (Variables|Default|SetDeadEnemies (+ (Variables|Default|GetDeadEnemies) 1))
  (bind _outactors (Actor|GetAllActorsOfClass "/Game/Blueprints/Door.Door_C"))
  (for _array_element _outactors
    (if (== (Variables|/Game/Blueprints/Door.Door_C|GetDeadEnemies _array_element) (Variables|Default|GetDeadEnemies))
      (Default|Move _array_element))))

(event EventBeginPlay
  (bind _returnvalue (Game|GetCurrentLevelName true))
  (CallFunction|ChangeLevel (Utilities|String|StringToName _returnvalue)))

(fn ConstructionScript)

(fn CreatingSpawners
  (params (Data :type Array%20of%20Data%20for%20Creating%20Spawners%20Structures))
  (for _array_element Data
    (bind _returnvalue (Game|SpawnActorfromClass "/Game/Blueprints/MyBaseSpawner.MyBaseSpawner_C" (.transform _array_element) "Undefined" 0 0))
    (if (.ReturnValue (Utilities|Map|Find (Variables|Default|GetEnemies) (.spawnertype _array_element)))
      (Class|BaseSpawner|Init _returnvalue (.Value (Utilities|Map|Find (Variables|Default|GetEnemies) (.spawnertype _array_element))) (.waves _array_element) (.accountwaves _array_element) (.complexity _array_element))
      (else
        (bind _enemy (CallFunction|FactoryMethod (.spawnertype _array_element) (.transform _array_element)))
        (CallFunction|AttachEnemy (.spawnertype _array_element) _enemy _returnvalue (.waves _array_element) (.accountwaves _array_element) (.complexity _array_element))))))

(fn AttachEnemy
  (params (Type :type E_SpawnerType%20Enum :default "EShotgunEnemy") (Enemy :type Enemy%20Character%20Object%20Reference) (Spawner :type Base%20Spawner%20Object%20Reference) (Waves :type Integer) (AccountWaves :type Boolean) (Complexity :type E_LevelOfDifficulty%20Enum :default "EEasy"))
  (Utilities|Array|Add (Variables|/Script/Engine.Actor|GetTags Enemy) "InSpawner")
  (Variables|/Script/TopDownShooter.BaseCharacter|Setdies Enemy true)
  (Utilities|Map|Add (Variables|Default|GetEnemies) Type Enemy)
  (Class|BaseSpawner|Init Spawner Enemy Waves AccountWaves Complexity))

(fn CreateObservers
  (bind _returnvalue (Game|SpawnActorfromClass "/Game/Blueprints/Observers/Achievements.Achievements_C" (Transformation|GetWorldTransform (Variables|Default|GetDefaultSceneRoot)) "Undefined" 0 0))
  (Utilities|Array|Add (Variables|Default|GetObservers) _returnvalue))

(fn FactoryMethod
  (params (NewParam1 :type E_SpawnerType%20Enum :default "EShotgunEnemy") (NewParam :type Transform))
  (bind _locationsforenemiesinspawners (Variables|Default|GetLocationsForEnemiesInSpawners))
  (bind (_value _returnvalue) (Utilities|Map|Find _locationsforenemiesinspawners NewParam1))
  (bind _returnvalue_2 (Math|Transform|SelectTransform _value NewParam _returnvalue))
  (switch Utilities|FlowControl|Switch|SwitchonE_SpawnerType NewParam1
    (:EShotgunEnemy
      (bind _returnvalue_3 (Game|SpawnActorfromClass "/Game/Blueprints/Enemies/MyEnemyWithShotgun.MyEnemyWithShotgun_C" _returnvalue_2 "Undefined" 0 0))
      (return _returnvalue_3))
    (:ERifleEnemy
      (bind _returnvalue_4 (Game|SpawnActorfromClass "/Game/Blueprints/Enemies/MyEnemyWithRifle.MyEnemyWithRifle_C" _returnvalue_2 "Undefined" 0 0))
      (return _returnvalue_4))))

(fn GenerateHeroCharacter
  (params (Transform :type Transform))
  (bind _builder (Variables|Default|GetBuilder))
  (Default|CreateHeroCharacter _builder Transform)
  (Default|SetWeapon _builder)
  (Default|SetMaterial _builder)
  (Default|SetSuperPower _builder)
  (bind _character (Default|DispatchHeroCharacter _builder))
  (return _character))